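; 360 camera actor that captures the scene through six-direction scene capture rigs into 2k or 4k render targets, in mono or stereo.
; SetModeQuality spawns the captures with shared grading, Lumen and optional path tracing settings, and disables some Lumen screen-space effects via console commands.
; The construction script offsets stereo rigs by half the eye distance and assigns a matching post-process preview material.
; BeginPlay enables per-frame capture; EndPlay disables it.
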(event `self.ReceiveBeginPlay`
  (bind _scenecapturecomponent2d_array (`self.SceneCaptureComponent2D_Array`))
  ; /!\ Important settings please don't change. /!\
  (`self.Set Mode & Quality`)
  (switch `/Game/Easy360Camera/Blueprint/Others/E_MonoStereo` (`self.Capture Mode`)
    (:`NewEnumerator0`
      (for _array_element _scenecapturecomponent2d_array
        (set `SceneCaptureComponent.bCaptureEveryFrame` true _array_element)))
    (:`NewEnumerator1`
      (for _array_element_2 _scenecapturecomponent2d_array
        (set `SceneCaptureComponent.bCaptureEveryFrame` true _array_element_2))
      (for _array_element_3 (`self.SceneCaptureComponent2D_Stereo_Array`)
        (set `SceneCaptureComponent.bCaptureEveryFrame` true _array_element_3)))))

(event `self.ReceiveEndPlay`
  (params (EndPlayReason :type "EEndPlayReason Enum" :default "Destroyed"))
  ; /!\ Important settings please don't change. /!\
  (for _array_element (`self.SceneCaptureComponent2D_Array`)
    (set `SceneCaptureComponent.bCaptureEveryFrame` false _array_element))
  (switch `/Game/Easy360Camera/Blueprint/Others/E_MonoStereo` (`self.Capture Mode`)
    (:`NewEnumerator1`
      (for _array_element_2 (`self.SceneCaptureComponent2D_Stereo_Array`)
        (set `SceneCaptureComponent.bCaptureEveryFrame` false _array_element_2)))))

(fn `Set Mode & Quality`
  (bind _render_target_size (`self.Render Target Size`))
  (`KismetSystemLibrary.ExecuteConsoleCommand` "r.PathTracing.ProgressDisplay 0" null)
  (`KismetSystemLibrary.ExecuteConsoleCommand` "r.Lumen.ScreenProbeGather.ScreenTraces 0" null)
  (`KismetSystemLibrary.ExecuteConsoleCommand` "r.Lumen.ScreenProbeGather.ShortRangeAO 0" null)
  (switch `/Game/Easy360Camera/Blueprint/Others/E_MonoStereo` (`self.Capture Mode`)
    (:`NewEnumerator0`
      (switch `/Game/Easy360Camera/Blueprint/Others/E_RenderTargets_Size` _render_target_size
        (:`NewEnumerator0`
          (`self.Set Mono Render Targets` (`self.RenderTargets 2k Mono`)))
        (:`NewEnumerator1`
          (`self.Set Mono Render Targets` (`self.RenderTargets 4k Mono`)))))
    (:`NewEnumerator1`
      (switch `/Game/Easy360Camera/Blueprint/Others/E_RenderTargets_Size` _render_target_size
        (:`NewEnumerator0`
          (`self.Set Mono Render Targets` (`self.RenderTargets 2k Mono`))
          (`self.Set Stereo Render Targets` (`self.RenderTargets 2k Stereo`)))
        (:`NewEnumerator1`
          (`self.Set Mono Render Targets` (`self.RenderTargets 4k Mono`))
          (`self.Set Stereo Render Targets` (`self.RenderTargets 4k Stereo`)))))))

(fn `Set Mono Render Targets`
  (params (`Render Targets` :type "Array of TextureRenderTarget2D Object Reference"))
  (bind (_offset_r _offset_g _offset_b _offset_a) (break `LinearColor` (`self.Offset`)))
  (bind (_saturation_r _saturation_g _saturation_b _saturation_a) (break `LinearColor` (`self.Saturation`)))
  (bind (_contrast_r _contrast_g _contrast_b _contrast_a) (break `LinearColor` (`self.Contrast`)))
  (bind (_gain_r _gain_g _gain_b _gain_a) (break `LinearColor` (`self.Gain`)))
  (bind (_gamma_r _gamma_g _gamma_b _gamma_a) (break `LinearColor` (`self.Gamma`)))
  (for _index (range 6)
    (bind (_output_location _output_rotation) (`KismetMathLibrary.BreakTransform` (`|GetArrayItem` (`self.SceneCaptureComponent Transforms`) _index)))
    (bind _returnvalue (`AddComponent|NODE_AddSceneCaptureComponent2D-2` :`RelativeTransform` (`KismetMathLibrary.MakeTransform` (0.0 0.0 0.0) _output_rotation (0.0 0.0 0.0))))
    (set `SceneCaptureComponent2D.TextureTarget` (`|GetArrayItem` `Render Targets` _index) _returnvalue)
    (`KismetArrayLibrary.Array_Insert` (`self.SceneCaptureComponent2D_Array`) _returnvalue _index)
    (set `SceneCaptureComponent2D.PostProcessSettings` (make `PostProcessSettings` :`AutoExposureMethod` "AEM_Manual" :`WhiteTemp` (`self.White Balance`) :`WhiteTint` (`self.White Balance Tint`) :`ColorSaturation` (`KismetMathLibrary.MakeVector4` _saturation_r _saturation_g _saturation_b _saturation_a) :`ColorContrast` (`KismetMathLibrary.MakeVector4` _contrast_r _contrast_g _contrast_b _contrast_a) :`ColorGamma` (`KismetMathLibrary.MakeVector4` _gamma_r _gamma_g _gamma_b _gamma_a) :`ColorGain` (`KismetMathLibrary.MakeVector4` _gain_r _gain_g _gain_b _gain_a) :`ColorOffset` (`KismetMathLibrary.MakeVector4` _offset_r _offset_g _offset_b _offset_a) :`BloomIntensity` 0.0 :`DynamicGlobalIlluminationMethod` (`self.Global Illum Method`) :`LumenRayLightingMode` (`self.Lumen Ray Lighting Mode`) :`LumenSceneLightingQuality` (`self.Lumen Scene Lighting Quality`) :`LumenSceneDetail` (`self.Lumen Scene Detail`) :`LumenFinalGatherQuality` (`self.Final Gather Quality`) :`ReflectionMethod` (`self.Reflections Method`) :`LumenReflectionQuality` (`self.Lumen Reflections Quality`) :`LumenFrontLayerTranslucencyReflections` (`self.High Quality Translucency Reflections`) :`ScreenSpaceReflectionIntensity` (`self.SSR Intensity`) :`ScreenSpaceReflectionQuality` (`self.SSR Quality`) :`AmbientCubemapIntensity` 0.0 :`AutoExposureBias` (+ (`self.Exposure`) 10.0) :`AutoExposureMinBrightness` 1.0 :`AutoExposureMaxBrightness` 1.0 :`LensFlareIntensity` 0.0 :`VignetteIntensity` 0.0 :`MotionBlurAmount` 0.0) _returnvalue)
    (`self.Set Pathtracing` _returnvalue)
    (set `SceneCaptureComponent.bCaptureEveryFrame` (`self.Capture Every Frame ? (Heavy)`) _returnvalue)))

(fn `Set Pathtracing`
  (params (SceneCaptureComponent2D :type "SceneCaptureComponent2D Object Reference"))
  (if (`self.Use PathTracing`)
    (set `SceneCaptureComponent.ShowFlagSettings` (`self.PathTracing ON`) SceneCaptureComponent2D)
    (else
      (set `SceneCaptureComponent.ShowFlagSettings` (`self.PathTracing OFF`) SceneCaptureComponent2D))))

(fn `Set Stereo Render Targets`
  (params (`Render Targets` :type "Array of TextureRenderTarget2D Object Reference"))
  (bind (_offset_r _offset_g _offset_b _offset_a) (break `LinearColor` (`self.Offset`)))
  (bind (_saturation_r _saturation_g _saturation_b _saturation_a) (break `LinearColor` (`self.Saturation`)))
  (bind (_contrast_r _contrast_g _contrast_b _contrast_a) (break `LinearColor` (`self.Contrast`)))
  (bind (_gain_r _gain_g _gain_b _gain_a) (break `LinearColor` (`self.Gain`)))
  (bind (_gamma_r _gamma_g _gamma_b _gamma_a) (break `LinearColor` (`self.Gamma`)))
  (for _index (range 6)
    (bind (_output_location _output_rotation) (`KismetMathLibrary.BreakTransform` (`|GetArrayItem` (`self.SceneCaptureComponent Transforms`) _index)))
    (bind _returnvalue (`AddComponent|NODE_AddSceneCaptureComponent2D-4` :`RelativeTransform` (`KismetMathLibrary.MakeTransform` (0.0 0.0 0.0) _output_rotation (0.0 0.0 0.0))))
    (set `SceneCaptureComponent2D.TextureTarget` (`|GetArrayItem` `Render Targets` _index) _returnvalue)
    (`KismetArrayLibrary.Array_Insert` (`self.SceneCaptureComponent2D_Stereo_Array`) _returnvalue _index)
    (set `SceneCaptureComponent2D.PostProcessSettings` (make `PostProcessSettings` :`AutoExposureMethod` "AEM_Manual" :`WhiteTemp` (`self.White Balance`) :`WhiteTint` (`self.White Balance Tint`) :`ColorSaturation` (`KismetMathLibrary.MakeVector4` _saturation_r _saturation_g _saturation_b _saturation_a) :`ColorContrast` (`KismetMathLibrary.MakeVector4` _contrast_r _contrast_g _contrast_b _contrast_a) :`ColorGamma` (`KismetMathLibrary.MakeVector4` _gamma_r _gamma_g _gamma_b _gamma_a) :`ColorGain` (`KismetMathLibrary.MakeVector4` _gain_r _gain_g _gain_b _gain_a) :`ColorOffset` (`KismetMathLibrary.MakeVector4` _offset_r _offset_g _offset_b _offset_a) :`BloomIntensity` 0.0 :`DynamicGlobalIlluminationMethod` (`self.Global Illum Method`) :`LumenRayLightingMode` (`self.Lumen Ray Lighting Mode`) :`LumenSceneLightingQuality` (`self.Lumen Scene Lighting Quality`) :`LumenSceneDetail` (`self.Lumen Scene Detail`) :`LumenFinalGatherQuality` (`self.Final Gather Quality`) :`ReflectionMethod` (`self.Reflections Method`) :`LumenReflectionQuality` (`self.Lumen Reflections Quality`) :`LumenFrontLayerTranslucencyReflections` (`self.High Quality Translucency Reflections`) :`ScreenSpaceReflectionIntensity` (`self.SSR Intensity`) :`ScreenSpaceReflectionQuality` (`self.SSR Quality`) :`AmbientCubemapIntensity` 0.0 :`AutoExposureBias` (+ (`self.Exposure`) 10.0) :`AutoExposureMinBrightness` 1.0 :`AutoExposureMaxBrightness` 1.0 :`LensFlareIntensity` 0.0 :`VignetteIntensity` 0.0 :`MotionBlurAmount` 0.0) _returnvalue)
    (`self.Set Pathtracing` _returnvalue)
    (set `SceneCaptureComponent.bCaptureEveryFrame` (`self.Capture Every Frame ? (Heavy)`) _returnvalue)))

(fn `UserConstructionScript`
  (bind _camera_preview (`self.Camera_Preview`))
  (bind _camera_preview_2 (`self.Camera_Preview`))
  ;[1 1 1] Capture mode
  (`self.Set Mode & Quality`)
  (switch `/Game/Easy360Camera/Blueprint/Others/E_MonoStereo` (`self.Capture Mode`)
    (:`NewEnumerator0`
      (for _array_element (`self.SceneCaptureComponent2D_Array`)
        (`SceneComponent.K2_SetRelativeLocation` _array_element (0.0 0.0 0.0) false false))
      (`KismetArrayLibrary.Array_Clear` (`self.SceneCaptureComponent2D_Stereo_Array`))
      (switch `/Game/Easy360Camera/Blueprint/Others/E_RenderTargets_Size` (`self.Render Target Size`)
        (:`NewEnumerator0`
          (set `CameraComponent.PostProcessSettings` (make `PostProcessSettings` :`WeightedBlendables` (`self.PP Material Preview Camera Mono 2k`)) _camera_preview_2))
        (:`NewEnumerator1`
          (set `CameraComponent.PostProcessSettings` (make `PostProcessSettings` :`WeightedBlendables` (`self.PP Material Preview Camera Mono 4k`)) _camera_preview_2))))
    (:`NewEnumerator1`
      (`self.Set Mode & Quality`)
      (for _array_element_2 (`self.SceneCaptureComponent2D_Stereo_Array`)
        (`SceneComponent.K2_SetRelativeLocation` _array_element_2 (`KismetMathLibrary.MakeVector` 0.0 (/ (/ (`KismetMathLibrary.Conv_IntToDouble` (`self.Eye Distance Stereo (mm)`)) 10.0) 2.0)) false false))
      (for _array_element_3 (`self.SceneCaptureComponent2D_Array`)
        (`SceneComponent.K2_SetRelativeLocation` _array_element_3 (`KismetMathLibrary.MakeVector` 0.0 (* (/ (/ (`KismetMathLibrary.Conv_IntToDouble` (`self.Eye Distance Stereo (mm)`)) 10.0) 2.0) -1.0)) false false))
      (switch `/Game/Easy360Camera/Blueprint/Others/E_RenderTargets_Size` (`self.Render Target Size`)
        (:`NewEnumerator0`
          (set `CameraComponent.PostProcessSettings` (make `PostProcessSettings` :`WeightedBlendables` (`self.PP Material Preview Camera Stereo 2k`)) _camera_preview))
        (:`NewEnumerator1`
          (set `CameraComponent.PostProcessSettings` (make `PostProcessSettings` :`WeightedBlendables` (`self.PP Material Preview Camera Stereo 4k`)) _camera_preview))))))